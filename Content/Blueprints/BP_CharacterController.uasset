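; Character controller Blueprint that shows a debug-style scoreboard when Tab is pressed.
; Tab calls the draw-score RPC, whose event walks the GameState PlayerArray and casts each entry to ProjectMPlayerState.
; Each player's ID and score are shown briefly with Print String rather than a UI widget.
; A failed cast stops the listing, and BeginPlay, Tick, overlap and construction hold no logic.
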(event Custom|RPC_DrawScore
  (for _array_element (Variables|/Script/Engine.GameStateBase|GetPlayerArray (Game|GetGameState))
    (bind _asproject_mplayer_state (Utilities|Casting|CastToProjectMPlayerState _array_element))
    (Development|PrintString (Utilities|String|ToString(Text) (Utilities|Text|FormatText "Player ID: {id}    Score: {score}" (Variables|/Script/Engine.PlayerState|GetPlayerId _asproject_mplayer_state) (Variables|/Script/ProjectM.ProjectMPlayerState|Get_score _asproject_mplayer_state))) true true "(R=0.000000,G=0.660000,B=1.000000,A=1.000000)" 5.0)))

(event EventBeginPlay)

(event Collision|EventActorBeginOverlap
  (params (OtherActor :type Actor%20Object%20Reference)))

(event EventTick
  (params (DeltaSeconds :type Float%20%28single-precision%29)))

(event Input|KeyboardEvents|Tab
  (params (Key :type Key%20Structure :default "None"))
  (:Pressed
    (CallFunction|RPCDrawScore)))

(fn ConstructionScript)