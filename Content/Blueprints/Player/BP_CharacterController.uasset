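; Player controller Blueprint that shows a scoreboard widget while Tab is held.
; Pressing Tab creates the widget, adds it to the viewport and stores it; releasing Tab removes it from the parent.
; Disconnected logic, which never runs, would toggle a respawn countdown from IsAlive on the local controller and ask ProjectMGameStateBase to show the end-game widget when no players remain alive.
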(event EventBeginPlay)

(event Collision|EventActorBeginOverlap
  (params (OtherActor :type Actor%20Object%20Reference)))

(event EventTick
  (params (DeltaSeconds :type Float%20%28single-precision%29)))

(event Input|KeyboardEvents|Tab
  (params (Key :type Key%20Structure :default "None"))
  (:Pressed
    (Utilities|IsValid (Variables|Default|GetScoreboard)
      (:Is%20Valid
        _)
      (:Is%20Not%20Valid
        _))
    (bind _returnvalue (UserInterface|CreateWidget "/Game/UI/Scoreboard.Scoreboard_C"))
    (UserInterface|Viewport|AddtoViewport _returnvalue 0)
    (Variables|Default|SetScoreboard _returnvalue))
  (:Released
    (Utilities|IsValid (Variables|Default|GetScoreboard)
      (:Is%20Valid
        (Widget|RemovefromParent (Variables|Default|GetScoreboard))))))

(fn ConstructionScript)